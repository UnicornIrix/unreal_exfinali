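; BP_cubozzoCangiante is a cube actor that gives itself a randomized look.
; Its construction script creates a dynamic instance of M_cubozzo on the Cube, picking one of five color variables at random, applying the Normal texture and rolling an emission between zero and MaxEmission.
; The event graph holds only disabled stub events, so it adds no runtime behavior.
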(fn `UserConstructionScript`
  (bind _returnvalue (`PrimitiveComponent.CreateDynamicMaterialInstance` (`self.Cube`) 0 "/Game/es_2/M_cubozzo.M_cubozzo" "None"))
  (bind _output_get (set `self.MI_cubozzo` _returnvalue))
  (`MaterialInstanceDynamic.SetVectorParameterValue` _output_get "Color" (`KismetArrayLibrary.Array_Random` (`|MakeArray` (`self.Color[ 0]`) (`self.Color[ 1]`) (`self.Color[ 2]`) (`self.Color[ 3]`) (`self.Color[ 4]`))))
  (`MaterialInstanceDynamic.SetTextureParameterValue` _output_get "Normal" (`self.Normal`))
  (`MaterialInstanceDynamic.SetScalarParameterValue` _output_get "Emission" (`KismetMathLibrary.RandomFloatInRange` 0.0 (`self.MaxEmission`))))